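; Test game mode that rewards player kills and can spawn tracker bots.
; On BeginPlay it binds to OnActorKilled, adding score to the killer's SPlayerState and printing it when a BP_PlayerPawn kills a non-player pawn, so teamkills earn nothing.
; SpawnNewBot, not called within this Blueprint, runs an EQS spawn-location query, then draws a debug sphere and attempts a BP_TrackerBot spawn at each returned location.
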(event Custom|OnQueryFinishedEvent_Event
  (params (QueryInstance :type Env%20Query%20Instance%20Blueprint%20Wrapper%20Object%20Reference) (QueryStatus :type EEnvQueryStatus%20Enum :default "Processing"))
  (switch Utilities|FlowControl|Switch|SwitchonEEnvQueryStatus QueryStatus
    (:Success
      (bind _resultlocations (AI|EQS|GetQueryResultsasLocations QueryInstance))
      (for _array_element _resultlocations
        (Rendering|Debug|DrawDebugSphere _array_element 1e+02 12 "(R=1.000000,G=0.792030,B=0.061193,A=1.000000)" 2.0 2.0)
        (Game|SpawnActorfromClass "/Game/TrackerBot/BP_TrackerBot.BP_TrackerBot_C" (Math|Transform|MakeTransform _array_element) "AdjustIfPossibleButDontSpawnIfColliding" 0 0)))))

(event Custom|OnActorKilled_Event
  (params (VictimActor :type Actor%20Object%20Reference) (KillerActor :type Actor%20Object%20Reference) (KillerController :type Controller%20Object%20Reference))
  ;[1 1 1] Dont reward teamkilling
  (bind _aspawn (Utilities|Casting|CastToPawn VictimActor))
  (if (not (Pawn|IsPlayerControlled _aspawn))
    (Utilities|IsValid KillerController
      (:Is%20Valid
        (bind _asbp_player_pawn (Utilities|Casting|CastToBP_PlayerPawn (Pawn|GetControlledPawn KillerController)))
        (bind _assplayer_state (Utilities|Casting|CastToSPlayerState (Variables|/Script/Engine.Pawn|GetPlayerState _asbp_player_pawn)))
        (Class|SPlayerState|AddScore _assplayer_state 2e+01)
        (Development|PrintString (Utilities|String|ToString(Text) (Utilities|Text|ToText(Float) (Variables|/Script/Engine.PlayerState|GetScore _assplayer_state) "HalfToEven")) true true "(R=0.000000,G=1.000000,B=0.259194,A=1.000000)" 1e+01)))))

(event EventBeginPlay
  (EventDispatchers|AssignOnActorKilled (delegate Custom|OnActorKilled_Event)))

(event EventSpawnNewBot
  (bind _returnvalue (AI|EQS|RunEQSQuery "/Game/Blueprints/EQS_FindSpawnLocation.EQS_FindSpawnLocation" self "RandomBest25Pct"))
  (EventDispatchers|AssignOnQueryFinishedEvent _returnvalue (delegate Custom|OnQueryFinishedEvent_Event)))

(fn ConstructionScript)